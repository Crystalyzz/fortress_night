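; BpC_PlayerResources is a building system Blueprint that holds the player's resources and tracks which one is selected.
; Getters expose the private selection state, resolving the selected index against the keys of the Resources map.
; A lookup searches ResourceWidgets for a matching resource, though its only visible return reports failure even after a match.
; It has no active event logic, as BeginPlay and Tick are disabled.
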(event EventBeginPlay
  (|CallParentFunction) ; This node is disabled and will not be called.\nDrag off pins to build functionality.
)

(event EventTick
  (params (DeltaSeconds :type Float%20%28single-precision%29))
  (|CallParentFunction DeltaSeconds) ; This node is disabled and will not be called.\nDrag off pins to build functionality.
)

(fn GetSelectedIndex
  (return (Variables|Default|GetSelectedResourceIndex)))

(fn GetSelectedResource
  ;[1 1 1] 当前创建变量为私有变量，以上Get func都是为外部提供访问私有变量的接口
  (bind _keys (Utilities|Map|Keys (Variables|Default|GetResources)))
  (return (Utilities|Array|Get(acopy) _keys (Variables|Default|GetSelectedResourceIndex))))

(fn GetWidgetforResource
  (params (Resource :type Bp%20Master%20Resource%20Class%20Reference))
  (bind _array_element (Utilities|Array|ForEachLoopwithBreak (Variables|Default|GetResourceWidgets) :!label _label)
    (:LoopBody
      (if (== (Variables|/Game/BuildingSystem/widgets/W_Resource.W_Resource_C|GetResource _array_element) Resource)
        (LocalVariables|SetlocalFound _array_element)
        (goto _label Break)))
    (:Completed
      (return false 0))))