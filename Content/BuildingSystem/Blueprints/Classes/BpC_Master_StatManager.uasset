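; Base stat manager Blueprint that holds a map of stats, each with minimum, current and maximum values.
; SetUpStats removes one enum entry, re-sets every remaining stat to clamp and refresh it, then fires OnStatsSetUp.
; ModifyStat prints the current value and applies deltas through SetStat, which clamps and overwrites the map's struct entry.
; SetStat then calls UpdateStat, an empty hook intended for UI refresh; its Update input is unused.
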(event Custom|onStatsSetUp)

(event Custom|SetUpStats
  (bind _stats (Variables|Default|GetStats))
  (Utilities|Map|Remove _stats "NewEnumerator0")
  (bind _keys (Utilities|Map|Keys _stats))
  (for _array_element _keys
    (CallFunction|SetStat _array_element (.CurrentValue (CallFunction|GetStat _array_element)) true))
  (CallFunction|OnStatsSetUp))

(fn UpdateStat
  (params (Stat :type e_Stats%20Enum :default "NewEnumerator0")))

(fn GetStat
  (params (Stat :type e_Stats%20Enum :default "NewEnumerator0"))
  (bind _stats (Variables|Default|GetStats))
  (bind _value (Utilities|Map|Find _stats Stat))
  (return (Utilities|Struct|Breaks_StatValue _value) _value))

(fn SetStat
  (params (Stat :type e_Stats%20Enum :default "NewEnumerator0") (NewValue :type Integer) (Update? :type Boolean))
  (LocalVariables|SetLocal%20Stat Stat)
  (LocalVariables|SetLocal%20Value NewValue)
  ;[1 1 1] 判定要修改的状态是否在map中
  (bind _keys (Utilities|Map|Keys (Variables|Default|GetStats)))
  ;[1 1 1] 如果存在，则继续尝试修改值，如果不存在，就直接return
  (if (Utilities|Array|ContainsItem _keys (LocalVariables|GetLocal%20Stat))
    ;[1 1 1] 把新建的对象直接覆盖属性映射map
    (Utilities|Map|Add (Variables|Default|GetStats) (LocalVariables|GetLocal%20Stat) (Utilities|Struct|Makes_StatValue (.MinValue (Utilities|Struct|Breaks_StatValue (.StatValue (CallFunction|GetStat (LocalVariables|GetLocal%20Stat))))) (Math|Integer|Clamp(Integer) (LocalVariables|GetLocal%20Value) (.MinValue (Utilities|Struct|Breaks_StatValue (.StatValue (CallFunction|GetStat (LocalVariables|GetLocal%20Stat))))) (.MaxValue (Utilities|Struct|Breaks_StatValue (.StatValue (CallFunction|GetStat (LocalVariables|GetLocal%20Stat)))))) (.MaxValue (Utilities|Struct|Breaks_StatValue (.StatValue (CallFunction|GetStat (LocalVariables|GetLocal%20Stat)))))))
    ;[1 1 1] 前面的属性已经变更，这里直接调用update，UI层会重新取数据更新UI的
    (CallFunction|UpdateStat (LocalVariables|GetLocal%20Stat))
    (return)
    (else
      (return))))

(fn ModifyStat
  (params (Stat :type e_Stats%20Enum :default "NewEnumerator0") (By :type Integer))
  (bind _currentvalue (CallFunction|GetStat Stat))
  (Development|PrintString (Utilities|String|Append "CurrentValue" (Utilities|String|ToString(Integer) _currentvalue)))
  (if (!= By 0)
    (CallFunction|SetStat Stat (+ _currentvalue By) true)
    (return)
    (else
      (return))))