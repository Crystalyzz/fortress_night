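; Player building manager component that shows a preview of the selected building in Construction state; selecting one from Combat switches the player to Construction.
; It generates building widgets through the player's main widget, highlights the selection and respawns the preview when it changes.
; A looping timer moves the preview ahead of the follow camera, snapped to grid and yaw steps.
; Resource events update the preview's resource and whether it is affordable.
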(event Custom|Initialize
  (params (Player :type Third%20Person%20Character%20Object%20Reference))
  (Utilities|IsValid Player
    (:Is%20Valid
      (Variables|Default|SetPlayerCharacter Player)
      (Variables|Default|SetInitialized? true)
      (bind _createdwidgets (Default|GenerateBuildingWidgets (Variables|/Game/ThirdPersonBP/Blueprints/ThirdPersonCharacter.ThirdPersonCharacter_C|GetMainWidget (Variables|Default|GetPlayerCharacter)) self))
      (Variables|Default|SetBuildingWidgets _createdwidgets)
      ;[1 1 1] initailize中，无法确定玩家开始游戏的状态，如果是建造模式需要选择一个建筑
      (switch Utilities|FlowControl|Switch|Switchone_PlayerStates (Variables|/Game/ThirdPersonBP/Blueprints/ThirdPersonCharacter.ThirdPersonCharacter_C|GetState (Variables|Default|GetPlayerCharacter))
        (:NewEnumerator1
          (CallFunction|SelectCurrentBuilding true))))))

(event Custom|OnStopBuilding
  (if (Variables|Default|GetCurrentBuilding?)
    (Variables|Default|SetCurrentBuilding? false)
    (CallFunction|SelectCurrentBuilding false)
    (Utilities|IsValid (Variables|Default|GetCurrentBuilding)
      (:Is%20Valid
        (Utilities|Time|ClearandInvalidateTimerbyHandle (Variables|Default|GetBuildingTimerHandle))
        (Actor|DestroyActor (Variables|Default|GetCurrentBuilding))
        (Variables|Default|SetCurrentBuilding 0)))))

(event Custom|ChangeCurrentBuilding
  (Utilities|Time|ClearandInvalidateTimerbyHandle (Variables|Default|GetBuildingTimerHandle)) ; 停止计时器
  (Actor|DestroyActor (Variables|Default|GetCurrentBuilding))
  (Variables|Default|SetCurrentBuilding 0)
  (CallFunction|StartBuilding) ; 选择下一个建筑
)

(event Custom|StartBuilding
  (bind (_location _rotation) (CallFunction|GetBuildingPosandRot))
  (bind _returnvalue (Game|SpawnActorfromClass (Utilities|Array|Get(acopy) (Variables|Default|GetBuildings) (Variables|Default|GetSelectedBuildingIndex)) (Math|Transform|MakeTransform _location _rotation "1,1,1") "Undefined" 0 (Default|GetSelectedResource (Variables|/Game/ThirdPersonBP/Blueprints/ThirdPersonCharacter.ThirdPersonCharacter_C|GetBpC_PlayerResources (Variables|Default|GetPlayerCharacter))) 0))
  (bind _output_get (Variables|Default|SetCurrentBuilding _returnvalue))
  (Default|SetCanbeBuilt _output_get (.Out (CallFunction|CanBuildBuilding)))
  (bind _returnvalue_2 (Utilities|Time|SetTimerbyEvent (delegate Custom|BuildingTick) (Variables|Default|GetBuildingUpdateInterval) true))
  (Variables|Default|SetBuildingTimerHandle _returnvalue_2))

(event Custom|BuildingTick
  (bind (_location _rotation) (CallFunction|GetBuildingPosandRot))
  (Transformation|SetActorLocationAndRotation (Variables|Default|GetCurrentBuilding) _location _rotation))

(event Custom|OnStartBuilding
  (if (Variables|Default|GetCurrentBuilding?)
    (CallFunction|ChangeCurrentBuilding)
    (else
      (CallFunction|StartBuilding)))
  (Variables|Default|SetCurrentBuilding? true))

(event Custom|OnResourceChanged
  (bind _currentbuilding (Variables|Default|GetCurrentBuilding))
  (if (and (Variables|Default|GetCurrentBuilding?) (Variables|Default|GetInitialized?))
    (Utilities|IsValid _currentbuilding
      (:Is%20Valid
        (Default|ChangeResource _currentbuilding (Default|GetSelectedResource (Variables|/Game/ThirdPersonBP/Blueprints/ThirdPersonCharacter.ThirdPersonCharacter_C|GetBpC_PlayerResources (Variables|Default|GetPlayerCharacter))))
        (Default|SetCanbeBuilt _currentbuilding (.Out (CallFunction|CanBuildBuilding)))))))

(event Custom|OnResourceValueModified
  (params (Resource :type Bp%20Master%20Resource%20Class%20Reference))
  (bind _currentbuilding (Variables|Default|GetCurrentBuilding))
  (if (Math|Boolean|ANDBoolean (Variables|Default|GetCurrentBuilding?) (Variables|Default|GetInitialized?) (Utilities|IsValidClass Resource) (== Resource (Default|GetSelectedResource (Variables|/Game/ThirdPersonBP/Blueprints/ThirdPersonCharacter.ThirdPersonCharacter_C|GetBpC_PlayerResources (Variables|Default|GetPlayerCharacter)))))
    (Utilities|IsValid _currentbuilding
      (:Is%20Valid
        (Default|SetCanbeBuilt _currentbuilding (.Out (CallFunction|CanBuildBuilding)))))))

(fn WidgetforBuilding
  (params (Building :type Bp%20Master%20Building%20Class%20Reference))
  (bind _array_element (Utilities|Array|ForEachLoopwithBreak (Variables|Default|GetBuildingWidgets) :!label _label)
    (:LoopBody
      (if (== (Variables|/Game/BuildingSystem/widgets/W_Building.W_Building_C|GetBuilding _array_element) Building)
        (LocalVariables|SetlocalFound _array_element)
        (goto _label Break)))
    (:Completed
      (Utilities|IsValid (LocalVariables|GetlocalFound)
        (:Is%20Valid
          (return true (LocalVariables|GetlocalFound)))
        (:Is%20Not%20Valid
          (return false 0))))))

(fn GetCurrentBuildingInfo
  (return (.BuildingData (Utilities|GetClassDefaults (Utilities|Array|Get(acopy) (Variables|Default|GetBuildings) (Variables|Default|GetSelectedBuildingIndex))))))

(fn SelectCurrentBuilding
  (params (Select? :type Boolean))
  (bind _buildings (Variables|Default|GetBuildings))
  (bind _selectedbuildingindex (Variables|Default|GetSelectedBuildingIndex))
  (bind _output (Utilities|Array|Get(acopy) _buildings _selectedbuildingindex))
  (bind (_success_ _widget) (CallFunction|WidgetforBuilding _output))
  (if _success_
    (Default|SelectBuilding _widget Select?)
    (if Select?
      (CallFunction|OnStartBuilding) ; 开始建造建筑
      (return)
      (else
        (return)))
    (else
      (return))))

(fn SelectBuildingbyIndex
  (params (Index :type Integer))
  (bind _output_get (LocalVariables|SetlocalIndex Index))
  (if (Math|Integer|InRange(Integer) _output_get 0 (Utilities|Array|LastIndex (Variables|Default|GetBuildings)))
    (switch Utilities|FlowControl|Switch|Switchone_PlayerStates (Variables|/Game/ThirdPersonBP/Blueprints/ThirdPersonCharacter.ThirdPersonCharacter_C|GetState (Variables|Default|GetPlayerCharacter)) ; 基于玩家的状态会有不同的功能，战斗-->建造状态
      (:NewEnumerator0
        (Variables|Default|SetSelectedBuildingIndex (LocalVariables|GetlocalIndex))
        (Default|ChangeState (Variables|Default|GetPlayerCharacter) "NewEnumerator1")
        (return))
      (:NewEnumerator1
        (if (!= (LocalVariables|GetlocalIndex) (Variables|Default|GetSelectedBuildingIndex))
          (CallFunction|SelectCurrentBuilding false)
          (Variables|Default|SetSelectedBuildingIndex (LocalVariables|GetlocalIndex))
          (CallFunction|SelectCurrentBuilding true)
          (return)
          (else
            (return)))))
    (else
      (return))))

(fn ToGridLocation
  (params (In :type Vector))
  (bind (_x _y _z) (Math|Vector|BreakVector In))
  (bind _zgridsize (Variables|BuildingGrid|GetZGridSize))
  (bind _xgridsize (Variables|BuildingGrid|GetXGridSize))
  (bind _ygridsize (Variables|BuildingGrid|GetYGridSize))
  (return (Math|Vector|MakeVector (Math|Conversions|ToFloat(Integer) (* (Math|Float|Round (/ _x (Math|Conversions|ToFloat(Integer) _xgridsize))) _xgridsize)) (Math|Conversions|ToFloat(Integer) (* (Math|Float|Round (/ _y (Math|Conversions|ToFloat(Integer) _ygridsize))) _ygridsize)) (Math|Conversions|ToFloat(Integer) (* (Math|Float|Round (/ _z (Math|Conversions|ToFloat(Integer) _zgridsize))) _zgridsize)))))

(fn ToSnapRotation
  (params (In :type Float%20%28single-precision%29))
  (bind _rotationsnap (Variables|BuildingGrid|GetRotationSnap))
  (return (* (Math|Float|Round (/ In (Math|Conversions|ToFloat(Integer) _rotationsnap))) _rotationsnap)))

(fn GetPlayerLookatLocation
  (params (ForwardOffset :type Integer))
  (bind _playercharacter (Variables|Default|GetPlayerCharacter))
  (return (+ (Transformation|GetActorLocation _playercharacter) (* (Math|Vector|GetForwardVector (Variables|/Game/ThirdPersonBP/Blueprints/ThirdPersonCharacter.ThirdPersonCharacter_C|GetFollowCamera _playercharacter)) ForwardOffset))))

(fn GetBuildingPosandRot
  (return (+ (CallFunction|ToGridLocation (CallFunction|GetPlayerLookatLocation (Variables|BuildingGrid|GetForwardBuildingOffset))) (Variables|BuildingGrid|GetLocationOffset)) (Math|Rotator|MakeRotator 0.0 0.0 (Math|Conversions|ToFloat(Integer) (+ (CallFunction|ToSnapRotation (.Yaw (Math|Rotator|BreakRotator (Transformation|GetWorldRotation (Variables|/Game/ThirdPersonBP/Blueprints/ThirdPersonCharacter.ThirdPersonCharacter_C|GetFollowCamera (Variables|Default|GetPlayerCharacter)))))) (Variables|BuildingGrid|GetRotationOffset))))))

(fn CanBuildBuilding
  (bind _playercharacter (Variables|Default|GetPlayerCharacter))
  (bind _currentbuilding (Variables|Default|GetCurrentBuilding))
  (bind _bpc_playerresources (Variables|/Game/ThirdPersonBP/Blueprints/ThirdPersonCharacter.ThirdPersonCharacter_C|GetBpC_PlayerResources _playercharacter))
  (bind _resourceversions (Variables|/Game/BuildingSystem/Blueprints/Classes/Bp_Master_Building.Bp_Master_Building_C|GetResourceVersions _currentbuilding))
  (bind _out (Default|GetSelectedResource _bpc_playerresources))
  (bind _value (Utilities|Map|Find _resourceversions _out))
  (bind _requiredamount (Utilities|Struct|Breaks_BuildingResourceVersion _value))
  (Utilities|IsValid (Variables|Default|GetCurrentBuilding)
    (:Is%20Valid
      (return (>= (Default|GetResource _bpc_playerresources _out) _requiredamount) _out _requiredamount))
    (:Is%20Not%20Valid
      (return false 0 0))))